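; BP_Dusman is an enemy that chases the first player character and dies when its health runs out.
; A looping timer started at BeginPlay reissues AI MoveTo toward the player at a fixed interval.
; AnyDamage prints a debug message and subtracts damage from Can (health).
; At zero or below, it calls DusmanOldu on the BP_Yonetici manager to report the death, then destroys itself.
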(event `self.ReceiveBeginPlay`
  (`KismetSystemLibrary.K2_SetTimerDelegate` (delegate `kovala`) 0.5 true))

(event `kovala`
  (`|AIMoveTo` self (0.0 0.0 0.0) (`GameplayStatics.GetPlayerCharacter` 0)))

(event `self.ReceiveAnyDamage`
  (params (Damage :type "Float (single-precision)") (DamageType :type "DamageType Object Reference") (InstigatedBy :type "Controller Object Reference") (DamageCauser :type "Actor Object Reference"))
  (bind _can (`self.Can`))
  (`KismetSystemLibrary.PrintString` "hasar verdin")
  (set `self.Can` (- _can Damage))
  (if (<= _can 0.0)
    (bind _returnvalue (`GameplayStatics.GetActorOfClass` "/Game/BP_Yonetici.BP_Yonetici_C"))
    (`/Game/BP_Yonetici.DusmanOldu` _returnvalue)
    (`self.K2_DestroyActor`)))

(fn `UserConstructionScript`)
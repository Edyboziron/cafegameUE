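; BP_Dusman is an enemy that chases the player by reissuing AI MoveTo on a looping timer.
; Incoming damage lowers Can (health); at zero it notifies BP_Yonetici, increments the player's score and destroys itself.
; On death it also checks the SkorKayit save slot to record a high score.
; Overlapping the player applies damage and starts a looping timer with no event shown bound, cleared when overlap ends.
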(event `self.ReceiveBeginPlay`
  (`KismetSystemLibrary.K2_SetTimerDelegate` (delegate `kovala`) 0.5 true))

(event `kovala`
  (`|AIMoveTo` self (0.0 0.0 0.0) (`GameplayStatics.GetPlayerCharacter` 0)))

(event `self.ReceiveAnyDamage`
  (params (Damage :type "Float (single-precision)") (DamageType :type "DamageType Object Reference") (InstigatedBy :type "Controller Object Reference") (DamageCauser :type "Actor Object Reference"))
  (bind _can (`self.Can`))
  (`KismetSystemLibrary.PrintString` "hasar verdin")
  (set `self.Can` (- _can Damage))
  (if (<= _can 0.0)
    (bind _returnvalue (`GameplayStatics.GetActorOfClass` "/Game/BP/BP_Yonetici.BP_Yonetici_C"))
    (`/Game/BP/BP_Yonetici.DusmanOldu` _returnvalue)
    (`KismetSystemLibrary.PrintString` "ölüm sinyali gitti")
    (bind _asbp_first_person_character (cast `/Game/FirstPerson/Blueprints/BP_FirstPersonCharacter` (`GameplayStatics.GetPlayerCharacter` 0))
      (:`then`
        (bind _output_get (set `/Game/FirstPerson/Blueprints/BP_FirstPersonCharacter.Skor` (+ (`/Game/FirstPerson/Blueprints/BP_FirstPersonCharacter.Skor` _asbp_first_person_character) 1) _asbp_first_person_character))
        (`GameplayStatics.CreateSaveGameObject` "/Game/BP/SG_Skor.SG_Skor_C")
        (bind _returnvalue_2 (`GameplayStatics.LoadGameFromSlot` "SkorKayit"))
        (if (`KismetSystemLibrary.IsValid` _returnvalue_2)
          (bind _assg_skor (cast `/Game/BP/SG_Skor` _returnvalue_2)
            (:`then`
              (if (> _output_get (`/Game/BP/SG_Skor.EnYuksekSkor` _assg_skor))
                (set `/Game/BP/SG_Skor.EnYuksekSkor` (`/Game/FirstPerson/Blueprints/BP_FirstPersonCharacter.Skor` _asbp_first_person_character) _assg_skor)
                (`GameplayStatics.SaveGameToSlot` null "SkorKayit" :!label _label)))
            (:`CastFailed`
              (`KismetSystemLibrary.PrintString` "cast failed")))
          (else
            (`GameplayStatics.CreateSaveGameObject` "/Game/BP/SG_Skor.SG_Skor_C")
            (goto _label)))
        (`self.K2_DestroyActor`))
      (:`CastFailed`
        (`KismetSystemLibrary.PrintString` "cast failed")))))

(event `self.ReceiveActorBeginOverlap`
  (params (OtherActor :type "Actor Object Reference"))
  (bind _returnvalue (`KismetSystemLibrary.K2_SetTimerDelegate` :`Time` 1.0 :`bLooping` true))
  (bind _asbp_first_person_character (cast `/Game/FirstPerson/Blueprints/BP_FirstPersonCharacter` OtherActor))
  (`GameplayStatics.ApplyDamage` _asbp_first_person_character 20.0))

(event `self.ReceiveActorEndOverlap`
  (params (OtherActor :type "Actor Object Reference"))
  (`KismetSystemLibrary.K2_ClearAndInvalidateTimerHandle` (stale `self.ReceiveActorBeginOverlap` _returnvalue)))

(fn `UserConstructionScript`)